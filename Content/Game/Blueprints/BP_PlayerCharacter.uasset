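; Third-person shooter player character that moves, touch-looks, sprints, jumps, aims, fires a spawned rifle and throws impulse-launched grenades.
; Input actions share logic with Do/Undo events, so other callers can trigger them.
; SetCameraMode switches to controller-yaw eight-direction movement when aiming, shooting or forced, which blocks jumping, with HUD tips.
; Sprinting stops and blocks firing, aiming overrides sprint speed, and a timeline zooms the spring arm.
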(event `self.ReceiveBeginPlay`
  (`self.InitWeapon`)
  (bind _ashud_tps (cast `/Game/Game/UserInterface/HUD/HUD_TPS` (`PlayerController.GetHUD` (`GameplayStatics.GetPlayerController` 0))))
  (set `self.HUD Widget` (`/Game/Game/UserInterface/HUD/HUD_TPS.HUD_Widget` _ashud_tps)))

(event `InputAxis|MoveForward`
  (params (AxisValue :type "Float (single-precision)"))
  (bind (_returnvalue_roll _returnvalue_pitch _returnvalue_yaw) (`KismetMathLibrary.BreakRotator` (`self.GetControlRotation`)))
  (`self.AddMovementInput` (`KismetMathLibrary.GetForwardVector` (`KismetMathLibrary.MakeRotator` 0.0 0.0 _returnvalue_yaw)) AxisValue))

(event `InputAxis|MoveRight`
  (params (AxisValue :type "Float (single-precision)"))
  (bind (_returnvalue_roll _returnvalue_pitch _returnvalue_yaw) (`KismetMathLibrary.BreakRotator` (`self.GetControlRotation`)))
  (`self.AddMovementInput` (`KismetMathLibrary.GetRightVector` (`KismetMathLibrary.MakeRotator` 0.0 0.0 _returnvalue_yaw)) AxisValue))

(event `InputTouch`
  (params (Location :type "Vector Structure") (FingerIndex :type "ETouchIndex Enum"))
  (bind (_returnvalue_x _returnvalue_y) (`KismetMathLibrary.BreakVector` (- (`self.TouchStart`) Location)))
  (:`Pressed`
    (set `self.TouchStart` Location))
  (:`Moved`
    (`self.AddControllerPitchInput` (* (* _returnvalue_y (`self.TurnSpeed`) (`GameplayStatics.GetWorldDeltaSeconds`)) -1.0))
    (`self.AddControllerYawInput` (* (* _returnvalue_x (`self.TurnSpeed`) (`GameplayStatics.GetWorldDeltaSeconds`)) -1.0))
    (set `self.TouchStart` Location)))

(event `InputAxis|LookUp`
  (params (AxisValue :type "Float (single-precision)"))
  (`self.AddControllerPitchInput` AxisValue))

(event `InputAxis|LookRight`
  (params (AxisValue :type "Float (single-precision)"))
  (`self.AddControllerYawInput` AxisValue))

(event `DoSprint`
  (set `self.IsSprinting` true :!label _label)
  (`self.IA STOP FIRE`)
  (`self.CalMaxWalkSpeed` :!label _label_2))

(event `InputAction|Sprint`
  (params (Key :type "Key Structure"))
  (:`Pressed`
    (goto _label))
  (:`Released`
    (set `self.IsSprinting` false :!label _label_3)
    (goto _label_2)))

(event `UndoSprint`
  (goto _label_3))

(event `Do Jump`
  (bind _hud_widget (`self.HUD Widget`))
  (if (`self.bUseControllerRotationYaw`) :!label _label_4
    (`/Engine/EditorBlueprintResources/StandardMacros.IsValid` _hud_widget
      (:`Is Valid`
        (`/Game/Game/UserInterface/HUD/W_HUD.TIP` _hud_widget "8方向移动 状态下 不可跳跃 \n因为没素材qaq")))
    (else
      (`self.Jump`))))

(event `InputAction|Jump`
  (params (Key :type "Key Structure"))
  (:`Pressed`
    (goto _label_4))
  (:`Released`
    (`self.StopJumping` :!label _label_5)))

(event `Undo Jump`
  (goto _label_5))

(event `DoAim`
  (set `self.IsAniming` true :!label _label)
  (`self.CalMaxWalkSpeed`)
  (`self.Set Camera Mode` false)
  (bind (_direction _track) (`Timeline|Aim` :!label _label_2)
    (:`Update`
      (set `SpringArmComponent.TargetArmLength` (`KismetMathLibrary.Lerp` 175.0 60.0 _track) (`self.SpringArm`)))))

(event `InputAction|Aim`
  (params (Key :type "Key Structure"))
  (:`Pressed`
    (goto _label))
  (:`Released`
    (set `self.IsAniming` false :!label _label_3)
    (`self.CalMaxWalkSpeed`)
    (`self.Set Camera Mode` false)
    (goto _label_2 :!via `Reverse`)))

(event `UndoAim`
  (goto _label_3))

(event `DoFire`
  (bind _hud_widget (`self.HUD Widget`))
  (if (not (`self.IsSprinting`)) :!label _label_4
    (bind _weapon (`self.Weapon`)
      (:`then`
        (`/Game/Game/Blueprints/BP_Weapon_AR4.Fire` _weapon)
        (set `self.IsShooting` true)
        (`self.Set Camera Mode` false))
      (:`else`))
    (else
      (`/Engine/EditorBlueprintResources/StandardMacros.IsValid` _hud_widget
        (:`Is Valid`
          (`/Game/Game/UserInterface/HUD/W_HUD.TIP` _hud_widget "不能在[冲刺键]按下时开枪！"))))))

(event `InputAction|Fire`
  (params (Key :type "Key Structure"))
  (:`Pressed`
    (goto _label_4))
  (:`Released`
    (bind _weapon (`self.Weapon` :!label _label_5)
      (:`then`
        (`/Game/Game/Blueprints/BP_Weapon_AR4.Stop Fire` _weapon)
        (set `self.IsShooting` false)
        (`self.Set Camera Mode` false))
      (:`else`))))

(event `UndoFire`
  (goto _label_5))

(event `IA STOP FIRE`
  (goto _label_5))

(event `Do 8Dir`
  (`self.Set Camera Mode` true :!label _label_6))

(event `InputAction|Do8Dir`
  (params (Key :type "Key Structure"))
  (:`Pressed`
    (goto _label_6)))

(event `Do Throw`
  (bind _returnvalue (`|SpawnActorFromClass` "/Game/Game/Blueprints/BP_Grenade.BP_Grenade_C" (`SceneComponent.GetSocketTransform` (`self.Mesh`) "S_Gender" "RTS_World") "AdjustIfPossibleButDontSpawnIfColliding" "OverrideRootScale" null null :!label _label_7))
  (`PrimitiveComponent.AddImpulse` (`/Game/Game/Blueprints/BP_Grenade.SM_Gender` _returnvalue) (* (`SceneComponent.GetForwardVector` (`self.Camera`)) (`/Game/Game/Blueprints/BP_Grenade.Speed` _returnvalue)) "None" false))

(event `InputAction|ThrowG`
  (params (Key :type "Key Structure"))
  (:`Pressed`
    (goto _label_7)))

(fn `CalMaxWalkSpeed`
  (set `CharacterMovementComponent.MaxWalkSpeed` (`KismetMathLibrary.SelectFloat` 150.0 600.0 (or (not (`self.IsSprinting`)) (`self.IsAniming`))) (`self.CharacterMovement`)))

(fn `InitWeapon`
  (bind _returnvalue (`|SpawnActorFromClass` "/Game/Game/Blueprints/BP_Weapon_AR4.BP_Weapon_AR4_C" (`KismetMathLibrary.MakeTransform` (0.0 0.0 0.0)) "Undefined" "OverrideRootScale" null null))
  (bind _output_get (set `self.Weapon` _returnvalue))
  (`self.K2_AttachToComponent` _output_get (`self.Mesh`) "S_Weapon" "SnapToTarget" "SnapToTarget" "SnapToTarget" true))

(fn `Set Camera Mode`
  (params (ForseSet :type Boolean) (ForseVal :type Boolean))
  (bind _hud_widget (`self.HUD Widget`))
  (bind _hud_widget_2 (`self.HUD Widget`))
  (bind _hud_widget_3 (`self.HUD Widget`))
  (bind _hud_widget_4 (`self.HUD Widget`))
  (if ForseSet
    (set `CharacterMovementComponent.bOrientRotationToMovement` ForseVal (`self.CharacterMovement`))
    (bind _output_get (set `self.bUseControllerRotationYaw` (not ForseVal)))
    (if _output_get
      (`/Engine/EditorBlueprintResources/StandardMacros.IsValid` _hud_widget_4
        (:`Is Valid`
          (`/Game/Game/UserInterface/HUD/W_HUD.TIP` _hud_widget_4 "现在是 八方向运动模式")
          (set `SpringArmComponent.TargetArmLength` 300.0 (`self.SpringArm`))))
      (else
        (`/Engine/EditorBlueprintResources/StandardMacros.IsValid` _hud_widget_2
          (:`Is Valid`
            (`/Game/Game/UserInterface/HUD/W_HUD.TIP` _hud_widget_2 "现在是 默认运动模式")))))
    (elif (or (`self.IsAniming`) (`self.IsShooting`))
      (set `CharacterMovementComponent.bOrientRotationToMovement` false (`self.CharacterMovement`))
      (set `self.bUseControllerRotationYaw` true)
      (`/Engine/EditorBlueprintResources/StandardMacros.IsValid` _hud_widget_3
        (:`Is Valid`
          (`/Game/Game/UserInterface/HUD/W_HUD.TIP` _hud_widget_3 "现在是 八方向运动模式")))
      (else
        (set `CharacterMovementComponent.bOrientRotationToMovement` true (`self.CharacterMovement`))
        (set `self.bUseControllerRotationYaw` false)
        (`/Engine/EditorBlueprintResources/StandardMacros.IsValid` _hud_widget
          (:`Is Valid`
            (`/Game/Game/UserInterface/HUD/W_HUD.TIP` _hud_widget "现在是 默认运动模式")))))))

(fn `UserConstructionScript`)