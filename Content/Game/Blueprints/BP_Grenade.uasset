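; BP_Grenade is a timed grenade actor that explodes after a BoomTime delay from BeginPlay.
; At the mesh's location it spawns a scaled explosion particle and sound, then runs a zero-length multi sphere trace as a radius check.
; Each BP_Target hit receives BeBoom with the hit component, blast center and impact point, and the grenade sets a short lifespan to remove itself.
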(event `self.ReceiveBeginPlay`
  (bind _returnvalue (`SceneComponent.K2_GetComponentLocation` (`self.SM_Gender`)))
  (`KismetSystemLibrary.Delay` (`self.BoomTime`))
  (`GameplayStatics.SpawnEmitterAtLocation` "/Game/MobileStarterContent/Particles/P_Explosion.P_Explosion" (`SceneComponent.K2_GetComponentLocation` (`self.SM_Gender`)) (struct) (7.0 7.0 7.0))
  (`GameplayStatics.PlaySoundAtLocation` "/Game/MobileStarterContent/Audio/Explosion_Cue.Explosion_Cue" (`SceneComponent.K2_GetComponentLocation` (`self.SM_Gender`)) (struct) 2.0 1.0 0.0 null null null)
  (`|ExecutionSequence`
    (:`then_0`
      (bind (_outhits _returnvalue_2) (`KismetSystemLibrary.SphereTraceMulti` _returnvalue _returnvalue (`self.Radius`) "TraceTypeQuery3"))
      (if _returnvalue_2
        (for _array_element _outhits
          (bind (_bblockinghit _binitialoverlap _time _distance _location _impactpoint _normal _impactnormal _physmat _hitactor _hitcomponent) (`GameplayStatics.BreakHitResult` _array_element))
          (bind _asbp_target (cast `/Game/Game/Blueprints/BP_Target` _hitactor))
          (`/Game/Game/Blueprints/BP_Target.BeBoom` _asbp_target _hitcomponent (`SceneComponent.K2_GetComponentLocation` (`self.SM_Gender`)) _location))))
    (:`then_1`
      (`self.SetLifeSpan` 0.5))))

(fn `UserConstructionScript`)