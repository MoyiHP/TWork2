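; Third-person shooter game mode that runs a timed round and tracks the score.
; Tick counts the remaining time down by world delta seconds and calls GameEnd at zero, which adds the game-over widget to the viewport and pauses the game.
; AddScore switches on the hit body part, awarding more points for head hits than for body, arm or leg hits.
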(event `self.ReceiveTick`
  (params (DeltaSeconds :type "Float (single-precision)"))
  (`|ExecutionSequence`
    (:`then_0`
      ;[1 1 1] set time
      (bind _output_get (set `self.TimeRemaind` (- (`self.TimeRemaind`) (`GameplayStatics.GetWorldDeltaSeconds`))))
      (if (<= _output_get 0.0)
        (`self.GameEnd`)))))

(event `GameEnd`
  (bind _returnvalue (`|CreateWidget` "/Game/Game/UserInterface/GameEnd/W_GameEnd.W_GameEnd_C"))
  (`UserWidget.AddToViewport` _returnvalue 1)
  (`GameplayStatics.SetGamePaused` true))

(fn `AddScore`
  (params (Hit :type "/Game/Game/Data/E_TargetHit Enum" :default "NewEnumerator0"))
  (switch `/Game/Game/Data/E_TargetHit` Hit
    (:`NewEnumerator0`
      (set `self.Score` (+ (`self.Score`) 3)))
    (:`NewEnumerator1`
      (set `self.Score` (+ (`self.Score`) 1)))
    (:`NewEnumerator2`
      (set `self.Score` (+ (`self.Score`) 1)))
    (:`NewEnumerator3`
      (set `self.Score` (+ (`self.Score`) 1)))))

(fn `UserConstructionScript`)