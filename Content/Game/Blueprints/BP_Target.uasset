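; Breakable humanoid shooting target that awards score by body part hit from BP_Bullet or explosions via BeBoom.
; Each hit adds GameMode_TPS score, spawns BP_ScoreShow, reduces Health (head costs more) and knocks the part loose with a physics impulse.
; Arm and leg hits always act on the left-side component.
; At zero Health all parts simulate physics and the actor is destroyed after a delay; only bullet hits check Death.
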(event `self.ReceiveBeginPlay`
  (bind _asgame_mode_tps (cast `/Game/Game/Blueprints/GameMode_TPS` (`GameplayStatics.GetGameMode`)))
  (set `self.As Game Mode TPS` _asgame_mode_tps))

(event `self.ReceiveHit`
  (params (MyComp :type "PrimitiveComponent Object Reference") (Other :type "Actor Object Reference") (OtherComp :type "PrimitiveComponent Object Reference") (bSelfMoved :type Boolean) (HitLocation :type "Vector Structure") (HitNormal :type "Vector Structure") (NormalImpulse :type "Vector Structure") (Hit :type "HitResult Structure (by ref)"))
  (cast `/Game/Game/Blueprints/BP_Bullet` Other)
  (if (not (`self.Death`))
    (`self.SwitchOnTargetComponent` MyComp
      (:`Head`
        (`/Game/Game/Blueprints/GameMode_TPS.AddScore` (`self.As Game Mode TPS`) "NewEnumerator0")
        (`|SpawnActorFromClass` "/Game/Game/Blueprints/BP_ScoreShow.BP_ScoreShow_C" (`KismetMathLibrary.MakeTransform` HitLocation) "AlwaysSpawn" "OverrideRootScale" null 3 null)
        (set `self.Health` (- (`self.Health`) 3))
        (`self.HitComp` (`self.Head`) HitLocation HitNormal)
        (`self.CheckHealth`))
      (:`Body`
        (`/Game/Game/Blueprints/GameMode_TPS.AddScore` (`self.As Game Mode TPS`) "NewEnumerator1")
        (`|SpawnActorFromClass` "/Game/Game/Blueprints/BP_ScoreShow.BP_ScoreShow_C" (`KismetMathLibrary.MakeTransform` HitLocation) "AlwaysSpawn" "OverrideRootScale" null 1 null)
        (`/Engine/EditorBlueprintResources/StandardMacros.DecrementInt` (`self.Health`)
          (:`  `
            (`self.HitComp` (`self.Body`) HitLocation HitNormal)
            (`self.CheckHealth`))))
      (:`Arm`
        (`/Game/Game/Blueprints/GameMode_TPS.AddScore` (`self.As Game Mode TPS`) "NewEnumerator2")
        (`|SpawnActorFromClass` "/Game/Game/Blueprints/BP_ScoreShow.BP_ScoreShow_C" (`KismetMathLibrary.MakeTransform` HitLocation) "AlwaysSpawn" "OverrideRootScale" null 1 null)
        (`/Engine/EditorBlueprintResources/StandardMacros.DecrementInt` (`self.Health`)
          (:`  `
            (`self.HitComp` (`self.ArmL`) HitLocation HitNormal)
            (`self.CheckHealth`))))
      (:`Leg`
        (`/Game/Game/Blueprints/GameMode_TPS.AddScore` (`self.As Game Mode TPS`) "NewEnumerator3")
        (`|SpawnActorFromClass` "/Game/Game/Blueprints/BP_ScoreShow.BP_ScoreShow_C" (`KismetMathLibrary.MakeTransform` HitLocation) "AlwaysSpawn" "OverrideRootScale" null 1 null)
        (`/Engine/EditorBlueprintResources/StandardMacros.DecrementInt` (`self.Health`)
          (:`  `
            (`self.HitComp` (`self.LegL`) HitLocation HitNormal)
            (`self.CheckHealth`)))))))

(event `DieEvent`
  (`self.Die`)
  (`KismetSystemLibrary.RetriggerableDelay` 1.0)
  (`self.K2_DestroyActor`))

(event `BeBoom`
  (params (HitComponent :type "Object Object Reference") (BoomLocation :type "Vector Structure") (HitLocation :type "Vector Structure"))
  (`self.SwitchOnTargetComponent` HitComponent
    (:`Head`
      (`/Game/Game/Blueprints/GameMode_TPS.AddScore` (`self.As Game Mode TPS`) "NewEnumerator0")
      (`|SpawnActorFromClass` "/Game/Game/Blueprints/BP_ScoreShow.BP_ScoreShow_C" (`KismetMathLibrary.MakeTransform` (`SceneComponent.K2_GetComponentLocation` (`self.Head`))) "AlwaysSpawn" "OverrideRootScale" null 3 null)
      (set `self.Health` (- (`self.Health`) 3))
      (`self.HitComp` (`self.Head`) HitLocation (`KismetMathLibrary.Normal` (- (`SceneComponent.K2_GetComponentLocation` (`self.Head`)) BoomLocation)))
      (`self.CheckHealth`))
    (:`Body`
      (`/Game/Game/Blueprints/GameMode_TPS.AddScore` (`self.As Game Mode TPS`) "NewEnumerator1")
      (`|SpawnActorFromClass` "/Game/Game/Blueprints/BP_ScoreShow.BP_ScoreShow_C" (`KismetMathLibrary.MakeTransform` (`SceneComponent.K2_GetComponentLocation` (`self.Body`))) "AlwaysSpawn" "OverrideRootScale" null 1 null)
      (`/Engine/EditorBlueprintResources/StandardMacros.DecrementInt` (`self.Health`)
        (:`  `
          (`self.HitComp` (`self.Body`) HitLocation (`KismetMathLibrary.Normal` (- (`SceneComponent.K2_GetComponentLocation` (`self.Body`)) BoomLocation)))
          (`self.CheckHealth`))))
    (:`Arm`
      (`/Game/Game/Blueprints/GameMode_TPS.AddScore` (`self.As Game Mode TPS`) "NewEnumerator2")
      (`|SpawnActorFromClass` "/Game/Game/Blueprints/BP_ScoreShow.BP_ScoreShow_C" (`KismetMathLibrary.MakeTransform` (`SceneComponent.K2_GetComponentLocation` (`self.ArmL`))) "AlwaysSpawn" "OverrideRootScale" null 1 null)
      (`/Engine/EditorBlueprintResources/StandardMacros.DecrementInt` (`self.Health`)
        (:`  `
          (`self.HitComp` (`self.ArmL`) HitLocation (`KismetMathLibrary.Normal` (- (`SceneComponent.K2_GetComponentLocation` (`self.ArmL`)) BoomLocation)))
          (`self.CheckHealth`))))
    (:`Leg`
      (`/Game/Game/Blueprints/GameMode_TPS.AddScore` (`self.As Game Mode TPS`) "NewEnumerator3")
      (`|SpawnActorFromClass` "/Game/Game/Blueprints/BP_ScoreShow.BP_ScoreShow_C" (`KismetMathLibrary.MakeTransform` (`SceneComponent.K2_GetComponentLocation` (`self.LegL`))) "AlwaysSpawn" "OverrideRootScale" null 1 null)
      (`/Engine/EditorBlueprintResources/StandardMacros.DecrementInt` (`self.Health`)
        (:`  `
          (`self.HitComp` (`self.LegL`) HitLocation (`KismetMathLibrary.Normal` (- (`SceneComponent.K2_GetComponentLocation` (`self.LegL`)) BoomLocation)))
          (`self.CheckHealth`))))))

(fn `CheckHealth`
  (if (not (> (`self.Health`) 0))
    (set `self.Death` true)
    (`self.DieEvent`)))

(fn `Die`
  (set `self.Death` true)
  (`PrimitiveComponent.SetSimulatePhysics` (`self.Head`) true)
  (`PrimitiveComponent.SetSimulatePhysics` (`self.ArmL`) true)
  (`PrimitiveComponent.SetSimulatePhysics` (`self.Body`) true)
  (`PrimitiveComponent.SetSimulatePhysics` (`self.ArmR`) true)
  (`PrimitiveComponent.SetSimulatePhysics` (`self.LegL`) true)
  (`PrimitiveComponent.SetSimulatePhysics` (`self.LegR`) true))

(fn `HitComp`
  (params (InputPin :type "PrimitiveComponent Object Reference") (Location :type "Vector Structure") (ImpluseDir :type "Vector Structure"))
  (`PrimitiveComponent.SetSimulatePhysics` InputPin true)
  (`PrimitiveComponent.AddImpulseAtLocation` InputPin (* ImpluseDir (`self.ImpluseScale`)) Location "None")
  (`PrimitiveComponent.SetCollisionResponseToChannel` InputPin "ECC_Pawn" "ECR_Overlap")
  (return))

(fn `UserConstructionScript`)