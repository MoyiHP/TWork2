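; BP_Weapon_AR4 is an automatic rifle weapon that fires repeatedly until told to stop.
; Fire starts a looping timer at the ShootSpeed interval, and StopFire clears it through the stored handle.
; Each Shoot spawns a BP_Bullet at the S_Muzzle socket, along with a scaled-down explosion particle as muzzle flash and a firing sound.
; Recoil is applied as pitch input on player controller 0, regardless of who holds the weapon.
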(event `Fire`
  (bind _returnvalue (`KismetSystemLibrary.K2_SetTimerDelegate` (delegate `Shoot`) (`self.ShootSpeed`) true))
  (set `self.ShootHandle` _returnvalue))

(event `Shoot`
  (bind (_returnvalue_location _returnvalue_rotation) (`KismetMathLibrary.BreakTransform` (`SceneComponent.GetSocketTransform` (`self.SK_AR4`) "S_Muzzle" "RTS_World")))
  (bind _returnvalue (`SceneComponent.GetSocketTransform` (`self.SK_AR4`) "S_Muzzle" "RTS_World"))
  (`|SpawnActorFromClass` "/Game/Game/Blueprints/BP_Bullet.BP_Bullet_C" (`KismetMathLibrary.MakeTransform` _returnvalue_location _returnvalue_rotation) "Undefined" "OverrideRootScale" null null)
  (`GameplayStatics.SpawnEmitterAtLocation` "/Game/MobileStarterContent/Particles/P_Explosion.P_Explosion" (.location _returnvalue) (`KismetMathLibrary.MakeRotator` (.roll (.rotation _returnvalue)) (+ (.pitch (.rotation _returnvalue)) 90.0) (.yaw (.rotation _returnvalue))) (0.1 0.05 0.05))
  (`GameplayStatics.PlaySoundAtLocation` "/Game/Game/Sound/AR4_Shoot.AR4_Shoot" (.location (`SceneComponent.GetSocketTransform` (`self.SK_AR4`) "S_Muzzle" "RTS_World")) (struct) 1.5 10.0 0.0 null null null)
  (`PlayerController.AddPitchInput` (`GameplayStatics.GetPlayerController` 0) -0.2))

(event `Stop Fire`
  (if (`KismetSystemLibrary.K2_IsValidTimerHandle` (`self.ShootHandle`))
    (`KismetSystemLibrary.K2_ClearAndInvalidateTimerHandle` (`self.ShootHandle`))))

(fn `UserConstructionScript`)